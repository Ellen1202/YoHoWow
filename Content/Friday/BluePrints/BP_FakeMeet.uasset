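; BP_FakeMeet is an interactable actor that teleports through a fixed sequence of hard-coded locations as the player interacts with it.
; Its Sphere overlap shows or removes a W_Interaction widget for BP_ThirdPersonCharacter and gates the Interaction event.
; Nested boolean flags advance one teleport per interaction.
; The last step calls CallFinishMoveEnd, destroys the Sphere, then destroys the actor after a delay.
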(event `self.Sphere.OnComponentBeginOverlap`
  (params (OverlappedComponent :type "PrimitiveComponent Object Reference") (OtherActor :type "Actor Object Reference") (OtherComp :type "PrimitiveComponent Object Reference") (OtherBodyIndex :type Integer) (bFromSweep :type Boolean) (SweepResult :type "HitResult Structure (by ref)"))
  (cast `/Game/ThirdPerson/Blueprints/BP_ThirdPersonCharacter` OtherActor)
  (bind _returnvalue (`|CreateWidget` "/Game/Widgets/W_Interaction.W_Interaction_C"))
  (`UserWidget.AddToPlayerScreen` _returnvalue 0)
  (set `self.IsOverlap` true))

(event `self.Sphere.OnComponentEndOverlap`
  (params (OverlappedComponent :type "PrimitiveComponent Object Reference") (OtherActor :type "Actor Object Reference") (OtherComp :type "PrimitiveComponent Object Reference") (OtherBodyIndex :type Integer))
  (cast `/Game/ThirdPerson/Blueprints/BP_ThirdPersonCharacter` OtherActor)
  (`Widget.RemoveFromParent` (stale `self.Sphere.OnComponentBeginOverlap` _returnvalue))
  (set `self.IsOverlap` false))

(event `/Game/ThirdPerson/Blueprints/BP_Interaction.Interaction`
  (if (`self.IsOverlap`)
    (if (`self.FirstMove`)
      (if (`self.SecondMove`)
        (if (`self.ThirdMove`)
          (if (`self.FinishMove`)
            (`self.K2_SetActorLocation` (-303.0 -3647.0 110.0) false true)
            (`self.FinishMoveEnd`)
            (`ActorComponent.K2_DestroyComponent` (`self.Sphere`))
            (`KismetSystemLibrary.Delay` 10.0)
            (`self.K2_DestroyActor`)
            (else
              (`self.K2_SetActorLocation` (-280.0 -3700.0 110.0) false true)
              (set `self.FinishMove` true)))
          (else
            (`self.K2_SetActorLocation` (546.0 -3813.0 110.0) false true)
            (set `self.ThirdMove` true)))
        (else
          (`self.K2_SetActorLocation` (670.0 -3881.0 110.0) false true)
          (set `self.SecondMove` true)))
      (else
        (`self.K2_SetActorLocation` (806.0 -3881.0 155.0) false true)
        (set `self.FirstMove` true)))))

(fn `UserConstructionScript`)