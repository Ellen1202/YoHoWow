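; BP_Chocolate is an interactable chocolate pickup that shows W_Interaction while the third-person character overlaps its sphere.
; Interaction calls EatChocolate while overlapping, then a DoOnce plays a find sound, removes the prompt and runs Seq_Chocolate in cinematic mode.
; After a delay matching the sequence's end time, it opens UMG_Chocolate with the mouse cursor shown, keeping movement and turning locked.
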(event `self.Sphere.OnComponentBeginOverlap`
  (params (OverlappedComponent :type "PrimitiveComponent Object Reference") (OtherActor :type "Actor Object Reference") (OtherComp :type "PrimitiveComponent Object Reference") (OtherBodyIndex :type Integer) (bFromSweep :type Boolean) (SweepResult :type "HitResult Structure (by ref)"))
  (cast `/Game/ThirdPerson/Blueprints/BP_ThirdPersonCharacter` OtherActor)
  (bind _returnvalue (`|CreateWidget` "/Game/Widgets/W_Interaction.W_Interaction_C"))
  (`UserWidget.AddToPlayerScreen` _returnvalue 0)
  (set `self.IsOverlap` true))

(event `self.Sphere.OnComponentEndOverlap`
  (params (OverlappedComponent :type "PrimitiveComponent Object Reference") (OtherActor :type "Actor Object Reference") (OtherComp :type "PrimitiveComponent Object Reference") (OtherBodyIndex :type Integer))
  (cast `/Game/ThirdPerson/Blueprints/BP_ThirdPersonCharacter` OtherActor)
  (`Widget.RemoveFromParent` (stale `self.Sphere.OnComponentBeginOverlap` _returnvalue))
  (set `self.IsOverlap` false))

(event `/Game/ThirdPerson/Blueprints/BP_Interaction.Interaction`
  (bind _returnvalue (`GameplayStatics.GetPlayerController` 0))
  (if (`self.IsOverlap`)
    (`self.EatChocolate`)
    (`/Engine/EditorBlueprintResources/StandardMacros.DoOnce` false
      (:`Completed`
        (`GameplayStatics.PlaySound2D` "/Game/Friday/SoundAssets/FindIt.FindIt" 1.0 1.0 0.0 null null)
        (`Widget.RemoveFromParent` (stale `self.Sphere.OnComponentBeginOverlap` _returnvalue))
        (bind (_outactor _returnvalue_2) (`LevelSequencePlayer.CreateLevelSequencePlayer` "/Game/Friday/Sequence/Seq_Chocolate.Seq_Chocolate"))
        (`MovieSceneSequencePlayer.SetPlaybackPosition` _returnvalue_2 (make `MovieSceneSequencePlaybackParams` (struct :`FrameNumber` (struct))))
        (`MovieSceneSequencePlayer.Play` _returnvalue_2)
        (`PlayerController.SetCinematicMode` (`GameplayStatics.GetPlayerController` 0) true true true true true)
        (`KismetSystemLibrary.Delay` (`TimeManagementBlueprintLibrary.Conv_QualifiedFrameTimeToSeconds` (`MovieSceneSequencePlayer.GetEndTime` _returnvalue_2)))
        (bind _returnvalue_3 (`|CreateWidget` "/Game/Friday/BluePrints/UMG_Chocolate.UMG_Chocolate_C"))
        (`UserWidget.AddToPlayerScreen` _returnvalue_3 0)
        (set `PlayerController.bShowMouseCursor` true _returnvalue)
        (`PlayerController.SetCinematicMode` _returnvalue true false true true true)))))

(fn `UserConstructionScript`)