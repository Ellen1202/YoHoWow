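; Interactable cup-shuffle (yabawi) minigame actor that the player starts through an overlap box and interaction prompt.
; Successive interactions fire dispatchers for zoom and animation, then open a three-choice widget once the shuffle ends.
; Parallel timelines reveal the middle cup, then slide the cups and Driver.
; The outcome is fixed: the first choice lifts the middle cup and sets the win flag, while the others lift losing cups with a beep.
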(event `self.Box.OnComponentBeginOverlap`
  (params (OverlappedComponent :type "PrimitiveComponent Object Reference") (OtherActor :type "Actor Object Reference") (OtherComp :type "PrimitiveComponent Object Reference") (OtherBodyIndex :type Integer) (bFromSweep :type Boolean) (SweepResult :type "HitResult Structure (by ref)"))
  (cast `/Game/ThirdPerson/Blueprints/BP_ThirdPersonCharacter` OtherActor)
  (bind _returnvalue (`|CreateWidget` "/Game/Widgets/W_Interaction.W_Interaction_C"))
  (`UserWidget.AddToPlayerScreen` _returnvalue 0)
  (set `self.IsOverlap` true))

(event `SelectedNumber1`
  (`GameplayStatics.PlaySound2D` "/Game/Friday/SoundAssets/Roulette.Roulette" 1.0 1.0 0.0 null null)
  (bind (_direction `_정답_보여주기`) (`Timeline|타임라인_1` :!via `PlayFromStart`)
    (:`Update`
      (`SceneComponent.K2_SetRelativeLocation` (`self.RedcupMiddle`) (`KismetMathLibrary.MakeVector` 0.0 20.0 `_정답_보여주기`) false false)
      (set `self.IsZoom?` false)
      (set `self.YabawiWin` true))))

(event `self.Box.OnComponentEndOverlap`
  (params (OverlappedComponent :type "PrimitiveComponent Object Reference") (OtherActor :type "Actor Object Reference") (OtherComp :type "PrimitiveComponent Object Reference") (OtherBodyIndex :type Integer))
  (cast `/Game/ThirdPerson/Blueprints/BP_ThirdPersonCharacter` OtherActor)
  (`Widget.RemoveFromParent` (stale `self.Box.OnComponentBeginOverlap` _returnvalue))
  (set `self.IsOverlap` false))

(event `SelectedNumber2`
  (`GameplayStatics.PlaySound2D` "/Game/Assets/Monday/BeepSound.BeepSound" 1.0 1.0 0.0 null null)
  (bind (_direction `_정답_보여주기`) (`Timeline|타임라인_0` :!via `PlayFromStart`)
    (:`Update`
      (`SceneComponent.K2_SetRelativeLocation` (`self.RedcupLeft`) (`KismetMathLibrary.MakeVector` 0.0 0.0 `_정답_보여주기`) false false)
      (set `self.IsZoom?` false))))

(event `/Game/ThirdPerson/Blueprints/BP_Interaction.Interaction`
  (if (`self.IsOverlap`)
    (if (`self.YabawiWin`)
      (`self.YaBaWi_Win`))
    (if (`self.IsZoom?`)
      (if (`self.IsAnimEnd`)
        (`Widget.RemoveFromParent` (stale `self.Box.OnComponentBeginOverlap` _returnvalue))
        (bind _returnvalue (`|CreateWidget` "/Game/Widgets/W_YaBaWiChoice.W_YaBaWiChoice_C"))
        (`UserWidget.AddToViewport` _returnvalue 0)
        (`|ExecutionSequence`
          (:`then_0`
            (add `/Game/Widgets/W_YaBaWiChoice.ClickedFirstChoice` _returnvalue (delegate `SelectedNumber1`)))
          (:`then_1`
            (add `/Game/Widgets/W_YaBaWiChoice.ClickedSecondChoice` _returnvalue (delegate `SelectedNumber2`)))
          (:`then_2`
            (add `/Game/Widgets/W_YaBaWiChoice.ClickedThirdChoice` _returnvalue (delegate `SelectedNumber3`))))
        (else
          (`self.PlayAnimation`)))
      (else
        (`self.CallRandomGame`)
        (`/Engine/EditorBlueprintResources/StandardMacros.DoOnce` false
          (:`Completed`
            (set `self.IsZoom?` true)))))))

(event `SelectedNumber3`
  (`GameplayStatics.PlaySound2D` "/Game/Assets/Monday/BeepSound.BeepSound" 1.0 1.0 0.0 null null)
  (bind (_direction `_정답_보여주기`) (`Timeline|타임라인` :!via `PlayFromStart`)
    (:`Update`
      (`SceneComponent.K2_SetRelativeLocation` (`self.RedcupRight`) (`KismetMathLibrary.MakeVector` 0.0 -20.0 `_정답_보여주기`) false false)
      (set `self.IsZoom?` false))))

(event `self.ReceiveBeginPlay`
  (add `self.PlayAnimation` (delegate `AnimEvent`)))

(event `AnimEvent`
  (if (not (`self.Clicked`))
    (set `self.Clicked` true)
    (`Widget.RemoveFromParent` (stale `self.Box.OnComponentBeginOverlap` _returnvalue))
    (bind (_direction `_정답_보여주기`) (`Timeline|Middle_Timeline` :!via `PlayFromStart`)
      (:`Update`
        (`SceneComponent.K2_SetRelativeLocation` (`self.RedcupMiddle`) (`KismetMathLibrary.MakeVector` 0.0 0.0 `_정답_보여주기`) false false)
        (`KismetSystemLibrary.Delay` 2.0)
        (`|ExecutionSequence`
          (:`then_0`
            (`GameplayStatics.PlaySound2D` "/Game/Friday/SoundAssets/Mix_Cup.Mix_Cup" 1.0 1.0 0.0 null null)
            (bind (_direction_2 _move) (`Timeline|Middle_Timeline2` :!via `PlayFromStart`)
              (:`Update`
                (`SceneComponent.K2_SetRelativeLocation` (`self.RedcupMiddle`) (`KismetMathLibrary.MakeVector` 0.0 _move 30.3) false false))))
          (:`then_1`
            (bind (_direction_3 _move_2) (`Timeline|Driver_Timeline` :!via `PlayFromStart`)
              (:`Update`
                (`SceneComponent.K2_SetRelativeLocation` (`self.Driver`) (`KismetMathLibrary.MakeVector` 0.0 _move_2 30.3) false false))
              (:`Finished`
                (set `self.IsAnimEnd` true)
                (`UserWidget.AddToPlayerScreen` (stale `self.Box.OnComponentBeginOverlap` _returnvalue) 0))))
          (:`then_2`
            (bind (_direction_4 _move_3) (`Timeline|Right_Timeline` :!via `PlayFromStart`)
              (:`Update`
                (`SceneComponent.K2_SetRelativeLocation` (`self.RedcupRight`) (`KismetMathLibrary.MakeVector` 0.0 _move_3 30.3) false false))))
          (:`then_3`
            (bind (_direction_5 _move_4) (`Timeline|Left_Timeline` :!via `PlayFromStart`)
              (:`Update`
                (`SceneComponent.K2_SetRelativeLocation` (`self.RedcupLeft`) (`KismetMathLibrary.MakeVector` 0.0 _move_4 30.3) false false)))))))))

(fn `UserConstructionScript`)