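; BP_Doll is an interactable doll actor that the player can use when standing inside its capsule.
; Capsule overlap with the third-person character shows or removes an interaction prompt widget and tracks whether the player is in range.
; When Interaction fires in range, it swaps the prompt for the doll UI and shows the mouse cursor.
; It then spawns an actor at a hardcoded location and destroys itself, making the interaction one-shot.
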(event `self.Capsule.OnComponentBeginOverlap`
  (params (OverlappedComponent :type "PrimitiveComponent Object Reference") (OtherActor :type "Actor Object Reference") (OtherComp :type "PrimitiveComponent Object Reference") (OtherBodyIndex :type Integer) (bFromSweep :type Boolean) (SweepResult :type "HitResult Structure (by ref)"))
  (cast `/Game/ThirdPerson/Blueprints/BP_ThirdPersonCharacter` OtherActor)
  (bind _returnvalue (`|CreateWidget` "/Game/Widgets/W_Interaction.W_Interaction_C"))
  (`UserWidget.AddToPlayerScreen` _returnvalue 0)
  (set `self.IsOverlap` true))

(event `self.Capsule.OnComponentEndOverlap`
  (params (OverlappedComponent :type "PrimitiveComponent Object Reference") (OtherActor :type "Actor Object Reference") (OtherComp :type "PrimitiveComponent Object Reference") (OtherBodyIndex :type Integer))
  (cast `/Game/ThirdPerson/Blueprints/BP_ThirdPersonCharacter` OtherActor)
  (`Widget.RemoveFromParent` (stale `self.Capsule.OnComponentBeginOverlap` _returnvalue))
  (set `self.IsOverlap` false))

(event `/Game/ThirdPerson/Blueprints/BP_Interaction.Interaction`
  (if (`self.IsOverlap`)
    (`Widget.RemoveFromParent` (stale `self.Capsule.OnComponentBeginOverlap` _returnvalue))
    (bind _returnvalue (`|CreateWidget` "/Game/Friday/BluePrints/UMG_Doll.UMG_Doll_C"))
    (`UserWidget.AddToPlayerScreen` _returnvalue 0)
    (set `PlayerController.bShowMouseCursor` true (`GameplayStatics.GetPlayerController` 0))
    (`|SpawnActorFromClass` "/Game/Friday/BluePrints/BP_FakeMeet.BP_FakeMeet_C" (`KismetMathLibrary.MakeTransform` (800.0 -4051.0 154.0)) "Undefined" "MultiplyWithRoot" null null)
    (`self.K2_DestroyActor`)))

(fn `UserConstructionScript`)