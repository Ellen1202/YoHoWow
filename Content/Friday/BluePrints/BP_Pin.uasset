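; BP_Pin is an interactable pin actor that the third-person character can find.
; Its capsule overlap with the character shows a W_Interaction widget and sets an overlap flag, both cleared on exit.
; When Interaction fires during an overlap, the pin teleports to a hardcoded location and rotation, marks itself found and calls CallFindPin, apparently to signal the discovery.
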(event `self.Capsule.OnComponentBeginOverlap`
  (params (OverlappedComponent :type "PrimitiveComponent Object Reference") (OtherActor :type "Actor Object Reference") (OtherComp :type "PrimitiveComponent Object Reference") (OtherBodyIndex :type Integer) (bFromSweep :type Boolean) (SweepResult :type "HitResult Structure (by ref)"))
  (cast `/Game/ThirdPerson/Blueprints/BP_ThirdPersonCharacter` OtherActor)
  (bind _returnvalue (`|CreateWidget` "/Game/Widgets/W_Interaction.W_Interaction_C"))
  (`UserWidget.AddToPlayerScreen` _returnvalue 0)
  (set `self.IsOverlap` true))

(event `self.Capsule.OnComponentEndOverlap`
  (params (OverlappedComponent :type "PrimitiveComponent Object Reference") (OtherActor :type "Actor Object Reference") (OtherComp :type "PrimitiveComponent Object Reference") (OtherBodyIndex :type Integer))
  (cast `/Game/ThirdPerson/Blueprints/BP_ThirdPersonCharacter` OtherActor)
  (`Widget.RemoveFromParent` (stale `self.Capsule.OnComponentBeginOverlap` _returnvalue))
  (set `self.IsOverlap` false))

(event `/Game/ThirdPerson/Blueprints/BP_Interaction.Interaction`
  (if (`self.IsOverlap`)
    (`self.K2_SetActorLocation` (490.0 -4200.0 300.0) false true)
    (`self.K2_SetActorRotation` (struct :`Yaw` -90.0))
    (set `self.Find` true)
    (`self.FindPin`)))

(fn `UserConstructionScript`)