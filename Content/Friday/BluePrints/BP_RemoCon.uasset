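; BP_RemoCon is an interactable remote controller that the third-person character can use while standing in its capsule.
; Capsule overlap sets the in-range flag and shows a W_Interaction prompt; leaving removes it and resets the material to White.
; Interaction, when in range, branches on the stored add-to-screen result to hide or show the prompt with a Red or White material, then calls CallCallBPRemocon.
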(event `self.Capsule.OnComponentBeginOverlap`
  (params (OverlappedComponent :type "PrimitiveComponent Object Reference") (OtherActor :type "Actor Object Reference") (OtherComp :type "PrimitiveComponent Object Reference") (OtherBodyIndex :type Integer) (bFromSweep :type Boolean) (SweepResult :type "HitResult Structure (by ref)"))
  (cast `/Game/ThirdPerson/Blueprints/BP_ThirdPersonCharacter` OtherActor)
  (set `self.IsOverlap` true)
  (bind _returnvalue (`|CreateWidget` "/Game/Widgets/W_Interaction.W_Interaction_C"))
  (bind _returnvalue_2 (`UserWidget.AddToPlayerScreen` _returnvalue 0)))

(event `self.Capsule.OnComponentEndOverlap`
  (params (OverlappedComponent :type "PrimitiveComponent Object Reference") (OtherActor :type "Actor Object Reference") (OtherComp :type "PrimitiveComponent Object Reference") (OtherBodyIndex :type Integer))
  (cast `/Game/ThirdPerson/Blueprints/BP_ThirdPersonCharacter` OtherActor)
  (set `self.IsOverlap` false)
  (`Widget.RemoveFromParent` (stale `self.Capsule.OnComponentBeginOverlap` _returnvalue))
  (`PrimitiveComponent.SetMaterial` (`self.SM_RemoteController`) 1 "/Game/Low_Poly_Furniture/Beds/White.White"))

(event `/Game/ThirdPerson/Blueprints/BP_Interaction.Interaction`
  (if (`self.IsOverlap`)
    (if (stale `self.Capsule.OnComponentBeginOverlap` _returnvalue_2)
      (`Widget.RemoveFromParent` (stale `self.Capsule.OnComponentBeginOverlap` _returnvalue))
      (`PrimitiveComponent.SetMaterial` (`self.SM_RemoteController`) 1 "/Game/Low_Poly_Furniture/Carpets/Red.Red")
      (else
        (`UserWidget.AddToPlayerScreen` (stale `self.Capsule.OnComponentBeginOverlap` _returnvalue) 0)
        (`PrimitiveComponent.SetMaterial` (`self.SM_RemoteController`) 1 "/Game/Low_Poly_Furniture/Beds/White.White")))
    (`self.CallBPRemocon`)))

(fn `UserConstructionScript`)