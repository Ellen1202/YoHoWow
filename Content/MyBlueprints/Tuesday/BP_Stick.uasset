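; BP_Stick is an interactable fight stick that opens an SF6 puzzle UI and slides out when solved.
; Its box overlap shows an interaction prompt to the player until solved, and Interaction opens the SF6UI widget with mouse-only UI input.
; BeginPlay creates that widget, binds its SF6Correct event to SpawnGold, and spawns a delayed TVSound at the TV.
; SpawnGold plays a sound, moves the FightStickColorID component along X, and sets the one-time Gold flag.
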(event `self.Box.OnComponentBeginOverlap`
  (params (OverlappedComponent :type "PrimitiveComponent Object Reference") (OtherActor :type "Actor Object Reference") (OtherComp :type "PrimitiveComponent Object Reference") (OtherBodyIndex :type Integer) (bFromSweep :type Boolean) (SweepResult :type "HitResult Structure (by ref)"))
  (if (not (`self.gold`))
    (cast `/Game/ThirdPerson/Blueprints/BP_ThirdPersonCharacter` OtherActor)
    (bind _returnvalue (`|CreateWidget` "/Game/Widgets/W_Interaction.W_Interaction_C"))
    (`UserWidget.AddToPlayerScreen` _returnvalue 0)))

(event `self.Box.OnComponentEndOverlap`
  (params (OverlappedComponent :type "PrimitiveComponent Object Reference") (OtherActor :type "Actor Object Reference") (OtherComp :type "PrimitiveComponent Object Reference") (OtherBodyIndex :type Integer))
  (cast `/Game/ThirdPerson/Blueprints/BP_ThirdPersonCharacter` OtherActor)
  (`Widget.RemoveFromParent` (stale `self.Box.OnComponentBeginOverlap` _returnvalue)))

(event `/Game/ThirdPerson/Blueprints/BP_Interaction.Interaction`
  (bind _returnvalue (`GameplayStatics.GetPlayerController` 0))
  (set `PlayerController.bShowMouseCursor` true _returnvalue)
  (`WidgetBlueprintLibrary.SetInputMode_UIOnlyEx` _returnvalue null)
  (`UserWidget.AddToViewport` (`self.SF6Stick`) 0))

(event `self.ReceiveBeginPlay`
  (`|ExecutionSequence`
    (:`then_0`
      (`KismetSystemLibrary.Delay` 1.5)
      (bind _returnvalue (`|SpawnActorFromClass` "/Game/MyBlueprints/Tuesday/TVSound.TVSound_C" (`SceneComponent.K2_GetComponentToWorld` (`Actor.RootComponent` (`self.TV`))) "Undefined" "MultiplyWithRoot" null null)))
    (:`then_1`
      (bind _returnvalue_2 (`|CreateWidget` "/Game/MyBlueprints/Tuesday/UI/SF6UI.SF6UI_C"))
      (bind _output_get (set `self.SF6Stick` _returnvalue_2))
      (add `/Game/MyBlueprints/Tuesday/UI/SF6UI.SF6Correct` _output_get (delegate `Spawn Gold`))
      (`self.destroySF6Sound`))))

(event `Spawn Gold`
  (bind _fightstick_color_id (`self.FightStick_Color_ID`))
  (bind (_relativelocation_x _relativelocation_y _relativelocation_z) (`KismetMathLibrary.BreakVector` (`SceneComponent.RelativeLocation` _fightstick_color_id)))
  (if (not (`self.gold`))
    (set `self.X` _relativelocation_x)
    (set `self.Y` _relativelocation_y)
    (set `self.Z` _relativelocation_z)
    (`|ExecutionSequence`
      (:`then_0`
        (`GameplayStatics.PlaySound2D` "/Engine/VREditor/Sounds/VR_teleport_Cue.VR_teleport_Cue" 1.0 1.0 0.0 null null)
        (`KismetSystemLibrary.MoveComponentTo` _fightstick_color_id (`KismetMathLibrary.MakeVector` (+ (`self.X`) 130.0) (`self.Y`) (`self.Z`)) (struct) false false 0.5)
        (set `self.gold` true)))))

(fn `UserConstructionScript`)