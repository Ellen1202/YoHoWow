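; BP_Chair is an interactable chair that slides to a new position when its Interaction event fires.
; A Box trigger adds an interaction tutorial widget to the screen while the third-person character overlaps it and removes it on exit.
; Interaction plays a timeline that lerps the chair's relative X and Y location and also relocates the Box high above, out of the way.
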(event `self.Box.OnComponentBeginOverlap`
  (params (OverlappedComponent :type "PrimitiveComponent Object Reference") (OtherActor :type "Actor Object Reference") (OtherComp :type "PrimitiveComponent Object Reference") (OtherBodyIndex :type Integer) (bFromSweep :type Boolean) (SweepResult :type "HitResult Structure (by ref)"))
  (cast `/Game/ThirdPerson/Blueprints/BP_ThirdPersonCharacter` OtherActor)
  (bind _returnvalue (`|CreateWidget` "/Game/Widgets/W_Interaction_Tutorial.W_Interaction_Tutorial_C"))
  (`UserWidget.AddToPlayerScreen` _returnvalue 0))

(event `self.Box.OnComponentEndOverlap`
  (params (OverlappedComponent :type "PrimitiveComponent Object Reference") (OtherActor :type "Actor Object Reference") (OtherComp :type "PrimitiveComponent Object Reference") (OtherBodyIndex :type Integer))
  (cast `/Game/ThirdPerson/Blueprints/BP_ThirdPersonCharacter` OtherActor)
  (`Widget.RemoveFromParent` (stale `self.Box.OnComponentBeginOverlap` _returnvalue)))

(event `/Game/ThirdPerson/Blueprints/BP_Interaction.Interaction`
  (bind (_direction _door) (`Timeline|타임라인`)
    (:`Update`
      (`SceneComponent.K2_SetRelativeLocation` (`self.Chair_A_Chair_A`) (`KismetMathLibrary.MakeVector` (`KismetMathLibrary.Lerp` 0.0 40.0 _door) (`KismetMathLibrary.Lerp` 0.0 -80.0 _door)) false false)
      (`SceneComponent.K2_SetRelativeLocation` (`self.Box`) (0.0 0.0 1000.0) false false))))

(fn `UserConstructionScript`)