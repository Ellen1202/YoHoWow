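; BP_Toy is an interactable chicken toy that shows a memo on first use and later a food screen.
; The first Interaction opens the UMG_Memo widget and switches to mouse-driven UI input, while later ones play a squeak sound and increment a counter.
; Tick watches that counter and, on the third squeak, opens UMG_Food in UI-only mode, then bumps the count so it triggers only once.
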(event `/Game/ThirdPerson/Blueprints/BP_Interaction.Interaction`
  (bind _returnvalue (`GameplayStatics.GetPlayerController` 0))
  (if (`self.IsMemoRead`)
    (`GameplayStatics.PlaySound2D` "/Game/Assets/Monday/ToyChickenSound.ToyChickenSound" 1.0 1.0 0.0 null null)
    (set `self.InteractionCount` (+ (`self.InteractionCount`) 1))
    (else
      (bind _returnvalue_2 (`|CreateWidget` "/Game/Assets/Monday/UMG_Memo.UMG_Memo_C"))
      (`UserWidget.AddToViewport` _returnvalue_2 0)
      (set `self.IsMemoRead` true)
      (set `PlayerController.bShowMouseCursor` true _returnvalue)
      (`WidgetBlueprintLibrary.SetInputMode_UIOnlyEx` _returnvalue null))))

(event `self.ReceiveTick`
  (params (DeltaSeconds :type "Float (single-precision)"))
  (bind _returnvalue (`GameplayStatics.GetPlayerController` 0))
  (if (== (`self.InteractionCount`) 3)
    (bind _returnvalue_2 (`|CreateWidget` "/Game/Assets/Monday/UMG_Food.UMG_Food_C"))
    (`UserWidget.AddToViewport` _returnvalue_2 0)
    (set `PlayerController.bShowMouseCursor` true _returnvalue)
    (`WidgetBlueprintLibrary.SetInputMode_UIOnlyEx` _returnvalue null)
    (set `self.InteractionCount` 4)))

(fn `UserConstructionScript`)