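; BP_Meat is a goal item that clears the stage when the player interacts with it.
; Tick plays the 위아래 (up-down) timeline, which drives the Meat component's relative location and spins the actor.
; Sphere overlap with BP_ThirdPersonCharacter toggles an interaction prompt and IsOverlap flag.
; While that flag is set, Interaction plays a sound, shows the M_StageClear widget and cursor, and locks movement and turning through cinematic mode.
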(event `self.ReceiveTick`
  (params (DeltaSeconds :type "Float (single-precision)"))
  (bind (_direction `_새_트랙_2`) (`Timeline|위아래`)
    (:`Update`
      (`SceneComponent.K2_SetRelativeLocation` (`self.Meat`) (`KismetMathLibrary.MakeVector` (.z `_새_트랙_2`)) false false)
      (`self.K2_AddActorWorldRotation` (struct :`Yaw` 3.0)))))

(event `self.Sphere.OnComponentBeginOverlap`
  (params (OverlappedComponent :type "PrimitiveComponent Object Reference") (OtherActor :type "Actor Object Reference") (OtherComp :type "PrimitiveComponent Object Reference") (OtherBodyIndex :type Integer) (bFromSweep :type Boolean) (SweepResult :type "HitResult Structure (by ref)"))
  (cast `/Game/ThirdPerson/Blueprints/BP_ThirdPersonCharacter` OtherActor)
  (bind _returnvalue (`|CreateWidget` "/Game/Widgets/W_Interaction.W_Interaction_C"))
  (`UserWidget.AddToPlayerScreen` _returnvalue 0)
  (set `self.IsOverlap` true))

(event `self.Sphere.OnComponentEndOverlap`
  (params (OverlappedComponent :type "PrimitiveComponent Object Reference") (OtherActor :type "Actor Object Reference") (OtherComp :type "PrimitiveComponent Object Reference") (OtherBodyIndex :type Integer))
  (cast `/Game/ThirdPerson/Blueprints/BP_ThirdPersonCharacter` OtherActor)
  (`Widget.RemoveFromParent` (stale `self.Sphere.OnComponentBeginOverlap` _returnvalue))
  (set `self.IsOverlap` false))

(event `self.Interaction`
  (bind _returnvalue (`GameplayStatics.GetPlayerController` 0))
  (if (`self.IsOverlap`)
    (`GameplayStatics.PlaySound2D` "/Game/Friday/SoundAssets/FindIt.FindIt" 1.0 1.0 0.0 null null)
    (`Widget.RemoveFromParent` (stale `self.Sphere.OnComponentBeginOverlap` _returnvalue))
    (bind _returnvalue_2 (`|CreateWidget` "/Game/Assets/Monday/M_StageClear.M_StageClear_C"))
    (`UserWidget.AddToPlayerScreen` _returnvalue_2 0)
    (set `PlayerController.bShowMouseCursor` true _returnvalue)
    (`PlayerController.SetCinematicMode` _returnvalue true false true true true)))

(fn `UserConstructionScript`)